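; WheelManager_BP tracks completion of the wheel puzzle in Room 3 and triggers its payoff.
; Each OnWheelComplete call increments CurrentIndex and compares it to TotalWheels.
; On a match it plays a 2D sound, drops the CeilingVent_BP, opens the HachetDoor_BP and prints "Safe Opened".
; Both target actors are found by class at that moment through GetActorOfClass.
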(event `/Game/Room3/OnWheelComplete_BPI.On Wheel Complete`
  (bind _result (`/Engine/EditorBlueprintResources/StandardMacros.IncrementInt` (`self.Current Index`))
    (:`  `
      (if (== _result (`self.Total Wheels`))
        (`GameplayStatics.PlaySound2D` null 1.0 1.0 0.0 null null)
        (bind _returnvalue (`GameplayStatics.GetActorOfClass` "/Game/Room3/CeilingVent_BP.CeilingVent_BP_C"))
        (`/Game/Room3/CeilingVent_BP.DropVent` _returnvalue)
        (bind _returnvalue_2 (`GameplayStatics.GetActorOfClass` "/Game/Room3/HachetDoor_BP.HachetDoor_BP_C"))
        (`/Game/Room3/HachetDoor_BP.Open Hachet` _returnvalue_2)
        (`KismetSystemLibrary.PrintString` "Safe Opened")))))

(fn `UserConstructionScript`)