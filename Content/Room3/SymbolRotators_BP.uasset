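; Rotating symbol wheel puzzle piece for Room 3 that the player turns toward a target position.
; StartInteract plays a timeline that yaws the symbol a quarter turn, ignoring input while it animates or once solved.
; On finish it advances a four-step index; a match with TargetIndex plays a sound, locks the wheel and notifies WheelManager.
; The match check is skipped when the index wraps to zero.
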(event `/Game/Interaction/Interaction_BPI.Start Interact`
  (bind (_wheel_rotator_roll _wheel_rotator_pitch _wheel_rotator_yaw) (`KismetMathLibrary.BreakRotator` (`self.Wheel Rotator`)))
  (if (`self.Is Solved?`)
    _
    (elif (not (`TimelineComponent.IsPlaying` (`self.Timeline`)))
      (bind (_direction _alpha) (`Timeline|Timeline` :!via `PlayFromStart`)
        (:`Update`
          (bind _returnvalue (`KismetMathLibrary.Lerp` _wheel_rotator_yaw (- _wheel_rotator_yaw 90.0) _alpha))
          (`SceneComponent.K2_SetRelativeRotation` (`self.Rotating symbol`) (`KismetMathLibrary.MakeRotator` 0.0 0.0 _returnvalue) false false))
        (:`Finished`
          (set `self.Wheel Rotator` (`KismetMathLibrary.MakeRotator` 0.0 0.0 _returnvalue))
          (bind _result (`/Engine/EditorBlueprintResources/StandardMacros.IncrementInt` (`self.RotateIndex`))
            (:`  `
              (bind _output_get (set `self.RotateIndex` _result))
              (if (>= _output_get 4)
                (set `self.RotateIndex` 0)
                (elif (== (`self.Target Index`) (`self.RotateIndex`))
                  (`GameplayStatics.PlaySound2D` null 1.0 1.0 0.0 null null)
                  (`KismetSystemLibrary.PrintString` "Solved!!" false true (struct :`R` 0.149126 :`G` 1.0 :`A` 1.0))
                  (set `self.Is Solved?` true)
                  (message `/Game/Room3/OnWheelComplete_BPI.On Wheel Complete` (`self.Wheel Manager`))
                  (else
                    (`KismetSystemLibrary.PrintString` "Wrong!!" false true (struct :`R` 1.0 :`G` 0.00438 :`A` 1.0))))))))))))

(fn `UserConstructionScript`)