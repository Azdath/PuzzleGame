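; Interactable puzzle picture in Room 2 that rotates in 45-degree steps until it reaches its target orientation.
; StartInteract plays the RotatePictures timeline to animate pitch, ignoring input while it plays or once solved.
; Each finished turn advances an index that wraps at eight, skipping the target check on wrap.
; A match plays a sound, locks the picture and notifies PuzzleManager; the construction script assigns the painting mesh.
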(event `/Game/Interaction/Interaction_BPI.Start Interact`
  (bind (_picture_rotation_roll _picture_rotation_pitch) (`KismetMathLibrary.BreakRotator` (`self.Picture rotation`)))
  (if (`self.Is Solved?`)
    _
    (elif (not (`TimelineComponent.IsPlaying` (`self.RotatePictures`)))
      (bind (_direction _alpha) (`Timeline|RotatePictures` :!via `PlayFromStart`)
        (:`Update`
          (bind _returnvalue (`KismetMathLibrary.Lerp` _picture_rotation_pitch (- _picture_rotation_pitch 45.0) _alpha))
          (`SceneComponent.K2_SetRelativeRotation` (`self.PuzzlePicture`) (`KismetMathLibrary.MakeRotator` 0.0 _returnvalue) false false))
        (:`Finished`
          (set `self.Picture rotation` (`KismetMathLibrary.MakeRotator` 0.0 _returnvalue))
          (bind _result (`/Engine/EditorBlueprintResources/StandardMacros.IncrementInt` (`self.Rotate Index`))
            (:`  `
              (bind _output_get (set `self.Rotate Index` _result))
              (if (>= _output_get 8)
                (set `self.Rotate Index` 0)
                (elif (== (`self.Target Index`) (`self.Rotate Index`))
                  (`GameplayStatics.PlaySound2D` null 1.0 1.0 0.0 null null)
                  (`KismetSystemLibrary.PrintString` "Solved!!" false true (struct :`R` 0.149126 :`G` 1.0 :`A` 1.0))
                  (set `self.Is Solved?` true)
                  (message `/Game/Room2/PuzzleCompletion_BPI.On Puzzle Complete` (`self.Puzzle Manager`))
                  (else
                    (`KismetSystemLibrary.PrintString` "Wrong!!" false true (struct :`R` 1.0 :`G` 0.00438 :`A` 1.0))))))))))))

(fn `UserConstructionScript`
  (`StaticMeshComponent.SetStaticMesh` (`self.PuzzlePicture`) (`self.PaintingMesh`)))